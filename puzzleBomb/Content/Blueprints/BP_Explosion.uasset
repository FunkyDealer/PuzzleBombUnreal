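; BP_Explosion is a short-lived explosion actor that triggers destruction on objects caught in its physical radius.
; Overlapping actors implementing BPI_destructible receive HandleDestruction with the bomb type, which SetBombType assigns.
; Tick clears the Usable flag, so only overlaps occurring before the first tick cause damage.
; Timers remove the radius component shortly after BeginPlay and expire the actor a few seconds later.
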(event OnComponentBeginOverlap(ExplosionRadiusPhysical)
  (params (OverlappedComponent :type Primitive%20Component%20Object%20Reference) (OtherActor :type Actor%20Object%20Reference) (OtherComp :type Primitive%20Component%20Object%20Reference) (OtherBodyIndex :type Integer) (bFromSweep :type Boolean) (SweepResult :type Hit%20Result%20Structure%20%28by%20ref%29))
  ;[1 1 1] overlap
  (if (Variables|Default|GetUsable)
    (if (Utilities|DoesObjectImplementInterface OtherActor "/Game/Blueprints/Interfaces/BPI_destructible.BPI_destructible_C")
      (bind _asbpi_destructible (Utilities|Casting|CastToBPI_destructible OtherActor))
      (Default|HandleDestruction _asbpi_destructible (Variables|Default|GetBombType)))))

(event Custom|DestroyComponent
  ;[1 1 1] timers
  (Components|DestroyComponent (Variables|Default|GetExplosionRadiusPhysical)))

(event EventBeginPlay
  ;[1 1 1] timers
  (Utilities|Time|SetTimerbyEvent (delegate Custom|DestroyComponent) 0.5)
  (Actor|SetLifeSpan 3.0))

(event EventTick
  (params (DeltaSeconds :type Float%20%28single-precision%29))
  (Variables|Default|SetUsable false))

(fn ConstructionScript)

(fn SetBombType
  (params (bombType :type E_BombType%20Enum :default "NewEnumerator0"))
  (Variables|Default|SetBombType bombType))