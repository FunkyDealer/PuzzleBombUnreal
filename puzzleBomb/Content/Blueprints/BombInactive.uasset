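; BombInactive is a bomb pickup that the player character collects by touching it.
; When its static mesh overlaps a Character_BP, it calls AddBomb on that character and destroys itself.
; On Tick, the mesh bobs up and down in fixed local steps, flipping an UpDown flag on exact relative-height matches rather than using a timeline.
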(event OnComponentBeginOverlap(StaticMesh)
  (params (OverlappedComponent :type Primitive%20Component%20Object%20Reference) (OtherActor :type Actor%20Object%20Reference) (OtherComp :type Primitive%20Component%20Object%20Reference) (OtherBodyIndex :type Integer) (bFromSweep :type Boolean) (SweepResult :type Hit%20Result%20Structure%20%28by%20ref%29))
  ;[1 1 1] Interaction with player
  (bind _ascharacter_bp (Utilities|Casting|CastToCharacter_BP OtherActor))
  (Default|AddBomb _ascharacter_bp)
  (Actor|DestroyActor))

(event EventTick
  (params (DeltaSeconds :type Float%20%28single-precision%29))
  ;[1 1 1] Bouncy
  (if (Variables|Default|GetUp/Down)
    (Transformation|AddLocalOffset (Variables|Default|GetStaticMesh) (Math|Vector|MakeVector 0.0 0.0 0.5) false false)
    (if (== (.z (Variables|/Script/Engine.SceneComponent|GetRelativeLocation (Variables|Default|GetStaticMesh))) 2e+01)
      (Variables|Default|SetUp/Down false))
    (else
      (Transformation|AddLocalOffset (Variables|Default|GetStaticMesh) (Math|Vector|MakeVector 0.0 0.0 -0.5) false false)
      (if (== (.z (Variables|/Script/Engine.SceneComponent|GetRelativeLocation (Variables|Default|GetStaticMesh))) 0.0)
        (Variables|Default|SetUp/Down true)))))

(fn ConstructionScript)