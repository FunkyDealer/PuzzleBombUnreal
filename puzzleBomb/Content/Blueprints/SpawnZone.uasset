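; SpawnZone is an actor that keeps up to three inactive bombs present inside its box area.
; A looping three-second timer started at BeginPlay prunes destroyed bombs from its tracked array, iterating in reverse for safe removal.
; It then spawns enough BP_BombInactive actors at random points within the Box component's bounds to restore the count.
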(event Custom|CheckBombs
  ;[1 1 1] Verify if Bomb exists, respawn a new one, delete old ones that dont exist anymore from memory
  (bind (_arrayindex _arrayelement) (Utilities|Array|ReverseforEachLoop (Variables|Default|GetBombs))
    (:LoopBody
      (Utilities|IsValid _arrayelement
        (:Is%20Not%20Valid
          (Utilities|Array|RemoveIndex (Variables|Default|GetBombs) _arrayindex))))
    (:Completed
      (CallFunction|RespawnBomb))))

(event Custom|RespawnBomb
  (bind _bombs (Variables|Default|GetBombs))
  (bind _box (Variables|Default|GetBox))
  (bind _returnvalue (Utilities|Array|Length _bombs))
  (bind (_origin _boxextent) (Collision|GetComponentBounds _box))
  ;[1 1 1] Create a new bomb in the memory.
  (if (< _returnvalue 3)
    (for _index (range 1 (- 3 _returnvalue))
      (bind _returnvalue_2 (Game|SpawnActorfromClass "/Game/Blueprints/BP_BombInactive.BP_BombInactive_C" (Math|Transform|MakeTransform (Math|Random|RandomPointinBoundingBox _origin _boxextent) "0, 0, 0" "1,1,1") "Undefined" 0 0))
      (Utilities|Array|Add (Variables|Default|GetBombs) _returnvalue_2))))

(event EventBeginPlay
  ;[1 1 1] Verify every 3 seconds if spawner has bombs.
  (Utilities|Time|SetTimerbyEvent (delegate Custom|CheckBombs) 3.0 true))

(fn ConstructionScript)